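; Player controller for a networked snowball game that manages the player's snowball ammo, HUD and death screen.
; Spawning a snowball spends one from the count, whose OnRep fires a change event on the local controller.
; The local controller creates the HUD on BeginPlay or possession.
; On death it swaps the HUD for a died-info widget and notifies BP_GameState.
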(event Custom|SpawnSnowball
  (params (SpawnTransform :type Transform%20%28by%20ref%29) (Owner :type Actor%20Object%20Reference))
  (if (>= (Variables|Default|GetSnowballsCurrentAmount) 1)
    (CallFunction|SetSnowballsAmount (- (Variables|Default|GetSnowballsCurrentAmount) 1))
    (Game|SpawnActorfromClass "/Game/MagicBattle/BP_Snowball.BP_Snowball_C" SpawnTransform "AdjustIfPossibleButAlwaysSpawn" "MultiplyWithRoot" Owner 0)))

(event Custom|SetSnowballsAmount
  (params (Snowballs :type Integer))
  (Variables|Default|SetSnowballsCurrentAmount Snowballs))

(event Custom|OnPlayerDied
  (if (Pawn|IsLocalController)
    (Widget|RemovefromParent (Variables|Default|GetPlayerHUD))
    (bind _returnvalue (UserInterface|CreateWidget "/Game/MagicBattle/Widgets/WBP_DiedInfo.WBP_DiedInfo_C" self))
    (UserInterface|Viewport|AddtoViewport _returnvalue 0)
    (CallFunction|NotifyPlayerDied)))

(event Custom|NotifyPlayerDied
  (Default|OnPlayerDied (.AsBP%20Game%20State (Utilities|Casting|CastToBP_GameState (Game|GetGameState)))))

(event EventPossess
  (params (PossessedPawn :type Pawn%20Object%20Reference))
  (if (Pawn|IsLocalPlayerController)
    (bind _returnvalue (UserInterface|CreateWidget "/Game/MagicBattle/Widgets/WBP_PlayerHUD.WBP_PlayerHUD_C" self))
    (bind _output_get (Variables|Default|SetPlayerHUD _returnvalue))
    (UserInterface|Viewport|AddtoViewport _output_get 0)))

(event EventBeginPlay
  (if (Pawn|IsLocalPlayerController)
    (bind _returnvalue (UserInterface|CreateWidget "/Game/MagicBattle/Widgets/WBP_PlayerHUD.WBP_PlayerHUD_C" self))
    (bind _output_get (Variables|Default|SetPlayerHUD _returnvalue))
    (UserInterface|Viewport|AddtoViewport _output_get 0)))

(fn ConstructionScript)

(fn OnRepSnowballsCurrentAmount
  (if (Pawn|IsLocalPlayerController)
    (Default|CallSnowballsAmountChanged)))