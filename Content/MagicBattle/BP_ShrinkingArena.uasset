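; BP_ShrinkingArena is an arena actor that shrinks horizontally once shrinking is started.
; On BeginPlay it binds an event to the game state's arena-shrink start, and its StartShrinking function sets the Shrinking flag.
; While that flag is set, Tick reduces the Arena component's relative X and Y scale by ShrinkSpeed times delta time, keeping Z unchanged, with no lower limit.
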(event EventTick
  (params (DeltaSeconds :type Float%20%28single-precision%29))
  (bind _arena (Variables|Default|GetArena))
  (bind _relativescale3d (Variables|/Script/Engine.SceneComponent|GetRelativeScale3D _arena))
  (bind (_x _y _z) (Math|Vector|BreakVector _relativescale3d))
  (if (Variables|Default|GetbShrinking)
    (bind _output_get (Variables|Default|SetCurrentFrameShrinkAmount (* DeltaSeconds (Variables|Default|GetShrinkSpeed))))
    (Transformation|SetRelativeScale3D _arena (Math|Vector|MakeVector (- _x _output_get) (- _y _output_get) _z))))

(event EventBeginPlay
  (EventDispatchers|BindEventtoStartArenaShrink (.AsBP%20Game%20State (Utilities|Casting|CastToBP_GameState (Game|GetGameState))) (EventDispatchers|CreateEvent :!event StartShrinking)))

(fn ConstructionScript)

(fn StartShrinking
  (Variables|Default|SetbShrinking true))